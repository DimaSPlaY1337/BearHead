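; BP_OverplapPlatform is a platform that travels between two relative locations, reversing its route when its Collider begins an overlap.
; A Timeline alpha lerps the Platform component from StartLocation, captured at BeginPlay, to EndLocation.
; Tick restarts the Timeline whenever the platform sits at StartLocation and otherwise keeps it playing.
; Overlap only swaps the two endpoints, so a platform resting at the far end sets off back.
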(event OnComponentBeginOverlap(collider)
  (params (OverlappedComponent :type Primitive%20Component%20Object%20Reference) (OtherActor :type Actor%20Object%20Reference) (OtherComp :type Primitive%20Component%20Object%20Reference) (OtherBodyIndex :type Integer) (bFromSweep :type Boolean) (SweepResult :type Hit%20Result%20Structure%20%28by%20ref%29))
  (Variables|Default|SetForChange (Variables|PlarformSettings|GetEndLocation))
  (Variables|PlarformSettings|SetEndLocation (Variables|PlarformSettings|GetStartLocation))
  (Variables|PlarformSettings|SetStartLocation (Variables|Default|GetForChange)))

(event EventBeginPlay
  (Variables|PlarformSettings|SetStartLocation (Variables|/Script/Engine.SceneComponent|GetRelativeLocation (Variables|Default|Getplatform))))

(event EventTick
  (params (DeltaSeconds :type Float%20%28single-precision%29))
  (if (Math|Vector|Equal(Vector) (Variables|/Script/Engine.SceneComponent|GetRelativeLocation (Variables|Default|Getplatform)) (Variables|PlarformSettings|GetStartLocation) 0.0001)
    (bind _platformalpha (Timeline|PlatformMovementTimeLine PlayFromStart)
      (:Update
        (Transformation|SetRelativeLocation (Variables|Default|Getplatform) (Math|Vector|Lerp(Vector) (Variables|PlarformSettings|GetStartLocation) (Variables|PlarformSettings|GetEndLocation) _platformalpha) false false)))
    (else
      (Timeline|PlatformMovementTimeLine Play))))

(fn ConstructionScript)